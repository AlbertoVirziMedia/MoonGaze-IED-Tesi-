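; Player melee weapon that deals damage and drives hit feedback on three enemy types.
; WeaponAttack enables the attack collider, applies damage and plays Wwise audio; Tick disables the collider outside attacks.
; Collider overlaps trigger surface-switched impact sounds, slow motion until overlap ends, camera shake, particles and knockback.
; While attacking, a per-tick line trace between two blade points passes the hit bone to enemies for physics-animated reactions and further knockback.
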(event `self.ReceiveActorBeginOverlap`
  (params (OtherActor :type "Actor Object Reference")))

(event `self.ReceiveBeginPlay`
  ;[1 1 1] Begin Play
  (`self.Set RefToMainCharacter`))

(event `self.ReceiveTick`
  (params (DeltaSeconds :type "Float (single-precision)"))
  ;[1 1 1] Event Tick
  (`self.Set NO Collision`)
  ;[1 1 1] Hit Trace
  (`self.HitTrace`)
  (if (not (`MainCharacter.bIsAttacking` (`self.RefToMainCharacter`)))
    (`PrimitiveComponent.SetCollisionEnabled` (`self.AttackCollider`) "NoCollision")))

(event `Set NO Collision`
  ;[1 1 1] Set No Collision
  (if (not (`MainCharacter.bIsAttacking` (`self.RefToMainCharacter`)))
    (`PrimitiveComponent.SetCollisionEnabled` (`self.AttackCollider`) "NoCollision")))

(event `Set RefToMainCharacter`
  ;[1 1 1] Set the Ref To Main Character
  (bind _asmain_character_bp (cast `/Game/Blueprint/MainCharacter/MainCharacter_BP` (`GameplayStatics.GetPlayerPawn` 0)))
  (set `self.RefToMainCharacter` _asmain_character_bp))

(event `self.WeaponAttack`
  ;[1 1 1] Weapon Attack
  (set `MainCharacter.bIsAttacking` true (`self.RefToMainCharacter`))
  (`PrimitiveComponent.SetCollisionEnabled` (`self.AttackCollider`) "QueryOnly")
  (`GameplayStatics.ApplyDamage` (stale `self.AttackCollider.OnComponentBeginOverlap` OtherActor) 10.0 null null "/Script/Engine.DamageType")
  ;[1 1 1] WWise Weapon Attack Sound
  (bind _returnvalue (`AkGameplayStatics.SpawnAkComponentAtLocation` "/Game/Audio/MainCharacter/Kria_Attack.Kria_Attack"))
  (`AkComponent.SetSwitch` _returnvalue "" "")
  (`AkGameObject.PostAssociatedAkEvent` :`self` _returnvalue))

(event `self.AttackCollider.OnComponentBeginOverlap`
  (params (OverlappedComponent :type "PrimitiveComponent Object Reference") (OtherActor :type "Actor Object Reference") (OtherComp :type "PrimitiveComponent Object Reference") (OtherBodyIndex :type Integer) (bFromSweep :type Boolean) (SweepResult :type "HitResult Structure (by ref)"))
  (bind (_bblockinghit _binitialoverlap _time _distance _location _impactpoint _normal _impactnormal _physmat _hitactor _hitcomponent) (`GameplayStatics.BreakHitResult` SweepResult))
  ;[1 1 1] Weapon Attack
  ;[1 1 1] Check Object Hit Physical Materia WWise Sound
  (`/Engine/EditorBlueprintResources/StandardMacros.IsValid` _hitcomponent
    (:`Is Valid`
      (bind _output_get (set `self.OverlappedComponentMaterial` (`MaterialInterface.GetPhysicalMaterial` (`PrimitiveComponent.GetMaterial` _hitcomponent 0)))))
    (:`Is Not Valid`
      _))
  (if (not (!= _output_get (`self.NullObject`)))
    (set `self.OverlappedComponentMaterial` (`MaterialInterface.GetPhysicalMaterial` (`PrimitiveComponent.GetMaterial` (`|GetArrayItem` (`self.K2_GetComponentsByClass` _hitactor "/Script/Engine.SkeletalMeshComponent")) 0))))
  (bind _returnvalue (`AkGameplayStatics.SpawnAkComponentAtLocation` "/Game/Audio/Weapon/Weapon_Hit.Weapon_Hit"))
  (`AkComponent.SetSwitch` _returnvalue "Surface_Type" (`KismetSystemLibrary.GetDisplayName` (`self.OverlappedComponentMaterial`)))
  (`AkGameObject.PostAssociatedAkEvent` :`self` _returnvalue)
  ;[1 1 1] Slow World time during attack
  (`GameplayStatics.SetGlobalTimeDilation` 0.4)
  ;[1 1 1] Play Camera Shake
  (`PlayerController.ClientStartCameraShake` :`self` (`MainCharacter.MainCharacterPlayerController` (`self.RefToMainCharacter`)) :`Shake` "/Script/Tesi.AttackCameraShake")
  (`|ExecutionSequence`
    (:`then_0`
      ;[1 1 1] Cast To EMCharacter and Spawn Particle
      (bind _asesploratori_melee_character_bp (cast `/Game/Blueprint/Enemy/Esploratori/Melee/EsploratoriMeleeCharacter_BP` OtherActor))
      (`/Game/Blueprint/Enemy/Esploratori/Melee/EsploratoriMeleeCharacter_BP.SpawnHitParticle` _asesploratori_melee_character_bp)
      ;[1 1 1] Normal Attack feedback (Enemy Knockback)
      (`/Game/Blueprint/Enemy/Esploratori/Melee/EsploratoriMeleeCharacter_BP.KnockBack` _asesploratori_melee_character_bp (* (`SceneComponent.GetForwardVector` (`Character.CapsuleComponent` _asesploratori_melee_character_bp)) -1000.0)))
    (:`then_1`
      ;[1 1 1] Cast To LCharacter and Spawn Particle
      (bind _asliocarpio_character_bp (cast `/Game/Blueprint/Enemy/Liocarpio/LiocarpioCharacter_BP` OtherActor))
      (`/Game/Blueprint/Enemy/Liocarpio/LiocarpioCharacter_BP.SpawnHitParticle` _asliocarpio_character_bp)
      (`/Game/Blueprint/Enemy/Liocarpio/LiocarpioCharacter_BP.KnockBack` _asliocarpio_character_bp (* (`self.GetActorForwardVector` _asliocarpio_character_bp) -1000.0)))
    (:`then_2`
      ;[1 1 1] Cast To Medusa and Spawn Particle
      (bind _asmedusa_character_bp (cast `/Game/Blueprint/Enemy/Meduse/MedusaCharacter_BP` OtherActor))
      (`/Game/Blueprint/Enemy/Meduse/MedusaCharacter_BP.SpawnParticle` _asmedusa_character_bp)
      (`/Game/Blueprint/Enemy/Meduse/MedusaCharacter_BP.Knock Back` _asmedusa_character_bp (* (`self.GetActorForwardVector` _asmedusa_character_bp) -1000.0)))))

(event `self.AttackCollider.OnComponentEndOverlap`
  (params (OverlappedComponent :type "PrimitiveComponent Object Reference") (OtherActor :type "Actor Object Reference") (OtherComp :type "PrimitiveComponent Object Reference") (OtherBodyIndex :type Integer))
  ;[1 1 1] Reset World time
  (`GameplayStatics.SetGlobalTimeDilation` 1.0))

(event `HitTrace`
  ;[1 1 1] HitTrace
  (if (`MainCharacter.bIsAttacking` (`self.RefToMainCharacter`))
    (bind (_outhit _returnvalue) (`KismetSystemLibrary.LineTraceSingle` :`Start` (`SceneComponent.K2_GetComponentLocation` (`self.LowHit`)) :`End` (`SceneComponent.K2_GetComponentLocation` (`self.HighHit`)) :`TraceChannel` "TraceTypeQuery1" :`DrawDebugType` "ForDuration"))
    (if _returnvalue
      (bind (_bblockinghit _binitialoverlap _time _distance _location _impactpoint _normal _impactnormal _physmat _hitactor _hitcomponent _hitbonename) (`GameplayStatics.BreakHitResult` _outhit))
      (set `self.BoneHit` _hitbonename)
      ;[1 1 1] Enemy Physics Anim
      (`|ExecutionSequence`
        (:`then_0`
          (bind _asesploratori_melee_character_bp (cast `/Game/Blueprint/Enemy/Esploratori/Melee/EsploratoriMeleeCharacter_BP` _hitactor))
          (bind _returnvalue_2 (/ _impactpoint 10.0))
          (`/Game/Blueprint/Enemy/Esploratori/Melee/EsploratoriMeleeCharacter_BP.KnockBack` _asesploratori_melee_character_bp _returnvalue_2)
          (set `/Game/Blueprint/Enemy/Esploratori/Melee/EsploratoriMeleeCharacter_BP.PhysicsAnim` true _asesploratori_melee_character_bp)
          (set `/Game/Blueprint/Enemy/Esploratori/Melee/EsploratoriMeleeCharacter_BP.BoneHit` (`self.BoneHit`) _asesploratori_melee_character_bp)
          (`/Game/Blueprint/Enemy/Esploratori/Melee/EsploratoriMeleeCharacter_BP.Physics Hit` _asesploratori_melee_character_bp))
        (:`then_1`
          (bind _asmedusa_character_bp (cast `/Game/Blueprint/Enemy/Meduse/MedusaCharacter_BP` _hitactor))
          (`/Game/Blueprint/Enemy/Meduse/MedusaCharacter_BP.Knock Back` _asmedusa_character_bp _returnvalue_2)
          (set `/Game/Blueprint/Enemy/Meduse/MedusaCharacter_BP.Physics Anim` true _asmedusa_character_bp)
          (set `/Game/Blueprint/Enemy/Meduse/MedusaCharacter_BP.Bone Hit` (`self.BoneHit`) _asmedusa_character_bp)
          (`/Game/Blueprint/Enemy/Meduse/MedusaCharacter_BP.Activate Physics Anim` _asmedusa_character_bp))
        (:`then_2`
          (bind _asliocarpio_character_bp (cast `/Game/Blueprint/Enemy/Liocarpio/LiocarpioCharacter_BP` _hitactor))
          (`/Game/Blueprint/Enemy/Liocarpio/LiocarpioCharacter_BP.KnockBack` _asliocarpio_character_bp _returnvalue_2)
          (set `/Game/Blueprint/Enemy/Liocarpio/LiocarpioCharacter_BP.PhysicsAnim` true _asliocarpio_character_bp)
          (set `/Game/Blueprint/Enemy/Liocarpio/LiocarpioCharacter_BP.BoneHit` (`self.BoneHit`) _asliocarpio_character_bp)
          (`/Game/Blueprint/Enemy/Liocarpio/LiocarpioCharacter_BP.Physics Hit` _asliocarpio_character_bp))))))

(fn `UserConstructionScript`)