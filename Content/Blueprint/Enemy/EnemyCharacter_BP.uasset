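; Enemy character Blueprint that damages the main character and plays a Wwise hit sound.
; While the Attacking flag is set, damage collider overlaps cast to MainCharacter_BP and apply fixed damage; nothing in this file sets the flag.
; Any capsule overlap spawns an Ak component at the mesh location and posts Weapon_Hit with the Surface_Type switch set to Esploratore.
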(event `self.ReceiveTick`
  (params (DeltaSeconds :type "Float (single-precision)")))

(event `self.DamageCollider.OnComponentBeginOverlap`
  (params (OverlappedComponent :type "PrimitiveComponent Object Reference") (OtherActor :type "Actor Object Reference") (OtherComp :type "PrimitiveComponent Object Reference") (OtherBodyIndex :type Integer) (bFromSweep :type Boolean) (SweepResult :type "HitResult Structure (by ref)"))
  ;[1 1 1] Apply Damage to Main Character
  (if (`self.bAttacking`)
    (bind _asmain_character_bp (cast `/Game/Blueprint/MainCharacter/MainCharacter_BP` OtherActor))
    (`GameplayStatics.ApplyDamage` _asmain_character_bp 10.0 null null "/Script/Engine.DamageType")))

(event `self.CapsuleComponent.OnComponentBeginOverlap`
  (params (OverlappedComponent :type "PrimitiveComponent Object Reference") (OtherActor :type "Actor Object Reference") (OtherComp :type "PrimitiveComponent Object Reference") (OtherBodyIndex :type Integer) (bFromSweep :type Boolean) (SweepResult :type "HitResult Structure (by ref)"))
  (bind _returnvalue (`AkGameplayStatics.SpawnAkComponentAtLocation` "/Game/Audio/MainCharacter/Weapon_Hit.Weapon_Hit" (`SceneComponent.K2_GetComponentLocation` (`self.Mesh`))))
  (`AkComponent.SetSwitch` _returnvalue "Surface_Type" "Esploratore")
  (`AkGameObject.PostAssociatedAkEvent` :`self` _returnvalue))

(fn `UserConstructionScript`)