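; Boss area-of-effect impact actor that spreads outward and hurts the player caught in it.
; Tick lerps the AOE component's scale toward a wide, flat target by a fixed per-frame alpha, so growth depends on frame rate.
; Overlapping MainCharacter_BP triggers damage, hit particles and knockback opposite its mesh's forward vector, gated by a DoOnce that any end overlap resets.
; A Destroy event removes the actor after a short delay.
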(event `self.ReceiveTick`
  (params (DeltaSeconds :type "Float (single-precision)"))
  (bind _aoe (`self.AOE`))
  (`SceneComponent.SetWorldScale3D` _aoe (`KismetMathLibrary.VLerp` (`SceneComponent.K2_GetComponentScale` _aoe) (20.0 20.0 1.0) 0.01)))

(event `self.AOE.OnComponentBeginOverlap`
  (params (OverlappedComponent :type "PrimitiveComponent Object Reference") (OtherActor :type "Actor Object Reference") (OtherComp :type "PrimitiveComponent Object Reference") (OtherBodyIndex :type Integer) (bFromSweep :type Boolean) (SweepResult :type "HitResult Structure (by ref)"))
  (bind _asmain_character_bp (cast `/Game/Blueprint/MainCharacter/MainCharacter_BP` OtherActor))
  (`/Engine/EditorBlueprintResources/StandardMacros.DoOnce` false :!label _label
    (:`Completed`
      (`GameplayStatics.ApplyDamage` _asmain_character_bp 20.0 null null "/Script/Engine.DamageType")
      (`/Game/Blueprint/MainCharacter/MainCharacter_BP.SpawnHitParticle` _asmain_character_bp "None")
      (`/Game/Blueprint/MainCharacter/MainCharacter_BP.KnockBack` _asmain_character_bp (* (`SceneComponent.GetForwardVector` (`Character.Mesh` _asmain_character_bp)) (-1.0 -1.0 0.0)))
      (set `/Game/Blueprint/MainCharacter/MainCharacter_BP.Kria_Enemies_Hits` self _asmain_character_bp)
      (`KismetSystemLibrary.PrintString` "ddd"))))

(event `self.AOE.OnComponentEndOverlap`
  (params (OverlappedComponent :type "PrimitiveComponent Object Reference") (OtherActor :type "Actor Object Reference") (OtherComp :type "PrimitiveComponent Object Reference") (OtherBodyIndex :type Integer))
  (goto _label :!via `Reset`))

(event `Destroy`
  (`KismetSystemLibrary.Delay` 3.0)
  (`self.K2_DestroyActor`))

(fn `UserConstructionScript`)