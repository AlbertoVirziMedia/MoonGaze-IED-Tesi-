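; Boss enemy character that turns toward the player and damages them through three body or weapon colliders.
; Tick smoothly interpolates yaw toward the cached player pawn while SetNewRotation is true.
; Each collider applies damage, hit particles and backward knockback to MainCharacter_BP, gated by a DoOnce that resets on overlap end.
; SpawnAOE spawns an impact actor at the AOESocket, oriented by the Lanterna collider, and immediately calls Destroy on it.
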(event `SetRefToMainCharacter`
  ;[1 1 1] SetRefToMainCharacter
  (set `self.RefToMainCharacterPawn` (`GameplayStatics.GetPlayerPawn` 0)))

(event `self.ReceiveBeginPlay`
  ;[1 1 1] Begin Play
  ;[1 1 1] SetRefToMainCharacter
  (`self.SetRefToMainCharacter`))

(event `self.ReceiveTick`
  (params (DeltaSeconds :type "Float (single-precision)"))
  ;[1 1 1] EventTick
  (if (`self.SetNewRotation`)
    (`self.K2_SetActorRotation` (`KismetMathLibrary.RInterpTo` (`self.K2_GetActorRotation`) (`KismetMathLibrary.MakeRotator` 0.0 0.0 (.yaw (`KismetMathLibrary.FindLookAtRotation` (`self.K2_GetActorLocation`) (`self.K2_GetActorLocation` (`self.RefToMainCharacterPawn`))))) (`GameplayStatics.GetWorldDeltaSeconds`) 2.0))))

(event `InterpRotationToMain`
  ;[1 1 1] SmoothRotation
)

(event `self.DamageCollider.OnComponentBeginOverlap`
  (params (OverlappedComponent :type "PrimitiveComponent Object Reference") (OtherActor :type "Actor Object Reference") (OtherComp :type "PrimitiveComponent Object Reference") (OtherBodyIndex :type Integer) (bFromSweep :type Boolean) (SweepResult :type "HitResult Structure (by ref)"))
  ;[1 1 1] Various Damage Collider
  (bind _asmain_character_bp (cast `/Game/Blueprint/MainCharacter/MainCharacter_BP` OtherActor))
  (bind _output_get (set `self.RefTo Main CharacterActor` _asmain_character_bp))
  (`/Engine/EditorBlueprintResources/StandardMacros.DoOnce` false :!label _label
    (:`Completed`
      (`GameplayStatics.ApplyDamage` _output_get 20.0 null null "/Script/Engine.DamageType")
      ;[1 1 1] Main Charater Reaction
      (`/Game/Blueprint/MainCharacter/MainCharacter_BP.SpawnHitParticle` _output_get "None")
      (`/Game/Blueprint/MainCharacter/MainCharacter_BP.KnockBack` _output_get (* (`SceneComponent.GetForwardVector` (`Character.Mesh` (`self.RefTo Main CharacterActor`))) (-1.0 -1.0 0.0)))
      (set `/Game/Blueprint/MainCharacter/MainCharacter_BP.Kria_Enemies_Hits` self _output_get))))

(event `self.DamageCollider.OnComponentEndOverlap`
  (params (OverlappedComponent :type "PrimitiveComponent Object Reference") (OtherActor :type "Actor Object Reference") (OtherComp :type "PrimitiveComponent Object Reference") (OtherBodyIndex :type Integer))
  ;[1 1 1] Various Damage Collider
  (goto _label :!via `Reset`))

(event `self.DamageColliderDx.OnComponentBeginOverlap`
  (params (OverlappedComponent :type "PrimitiveComponent Object Reference") (OtherActor :type "Actor Object Reference") (OtherComp :type "PrimitiveComponent Object Reference") (OtherBodyIndex :type Integer) (bFromSweep :type Boolean) (SweepResult :type "HitResult Structure (by ref)"))
  ;[1 1 1] Various Damage Collider
  (bind _asmain_character_bp (cast `/Game/Blueprint/MainCharacter/MainCharacter_BP` OtherActor))
  (bind _output_get (set `self.RefTo Main CharacterActor` _asmain_character_bp))
  (`/Engine/EditorBlueprintResources/StandardMacros.DoOnce` false :!label _label_2
    (:`Completed`
      (`GameplayStatics.ApplyDamage` _output_get 10.0 null null "/Script/Engine.DamageType")
      ;[1 1 1] Main Charater Reaction
      (`/Game/Blueprint/MainCharacter/MainCharacter_BP.SpawnHitParticle` _output_get "None")
      (`/Game/Blueprint/MainCharacter/MainCharacter_BP.KnockBack` _output_get (* (`SceneComponent.GetForwardVector` (`Character.Mesh` (`self.RefTo Main CharacterActor`))) (-1.0 -1.0 0.0)))
      (set `/Game/Blueprint/MainCharacter/MainCharacter_BP.Kria_Enemies_Hits` self _output_get))))

(event `self.DamageColliderDx.OnComponentEndOverlap`
  (params (OverlappedComponent :type "PrimitiveComponent Object Reference") (OtherActor :type "Actor Object Reference") (OtherComp :type "PrimitiveComponent Object Reference") (OtherBodyIndex :type Integer))
  ;[1 1 1] Various Damage Collider
  (goto _label_2 :!via `Reset`))

(event `self.DamageColliderLanterna.OnComponentBeginOverlap`
  (params (OverlappedComponent :type "PrimitiveComponent Object Reference") (OtherActor :type "Actor Object Reference") (OtherComp :type "PrimitiveComponent Object Reference") (OtherBodyIndex :type Integer) (bFromSweep :type Boolean) (SweepResult :type "HitResult Structure (by ref)"))
  ;[1 1 1] Various Damage Collider
  (bind _asmain_character_bp (cast `/Game/Blueprint/MainCharacter/MainCharacter_BP` OtherActor))
  (bind _output_get (set `self.RefTo Main CharacterActor` _asmain_character_bp))
  (`/Engine/EditorBlueprintResources/StandardMacros.DoOnce` false :!label _label_3
    (:`Completed`
      (`GameplayStatics.ApplyDamage` _output_get 10.0 null null "/Script/Engine.DamageType")
      ;[1 1 1] Main Charater Reaction
      (`/Game/Blueprint/MainCharacter/MainCharacter_BP.SpawnHitParticle` _output_get "None")
      (`/Game/Blueprint/MainCharacter/MainCharacter_BP.KnockBack` _output_get (* (`SceneComponent.GetForwardVector` (`Character.Mesh` (`self.RefTo Main CharacterActor`))) (-1.0 -1.0 0.0)))
      (set `/Game/Blueprint/MainCharacter/MainCharacter_BP.Kria_Enemies_Hits` self _output_get))))

(event `self.DamageColliderLanterna.OnComponentEndOverlap`
  (params (OverlappedComponent :type "PrimitiveComponent Object Reference") (OtherActor :type "Actor Object Reference") (OtherComp :type "PrimitiveComponent Object Reference") (OtherBodyIndex :type Integer))
  ;[1 1 1] Various Damage Collider
  (goto _label_3 :!via `Reset`))

(fn `SpawnAOE`
  (bind _returnvalue (`|SpawnActorFromClass` "/Game/Blueprint/Enemy/Boss/aoeimpact_BP.aoeimpact_BP_C" (`KismetMathLibrary.MakeTransform` (`SceneComponent.GetSocketLocation` (`self.Mesh`) "AOESocket") (`KismetMathLibrary.MakeRotator` (- (.roll (.rotation (`SceneComponent.K2_GetComponentToWorld` (`self.DamageColliderLanterna`)))) 90.0) (.pitch (.rotation (`SceneComponent.K2_GetComponentToWorld` (`self.DamageColliderLanterna`)))) (.yaw (.rotation (`SceneComponent.K2_GetComponentToWorld` (`self.DamageColliderLanterna`))))) (.scale (`SceneComponent.K2_GetComponentToWorld` (`self.DamageColliderLanterna`)))) "Undefined" "OverrideRootScale" null null))
  (`/Game/Blueprint/Enemy/Boss/aoeimpact_BP.Destroy` _returnvalue))

(fn `UserConstructionScript`)