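; Medusa enemy character that damages and knocks back the main character when its damage collider overlaps them.
; BeginPlay configures physical animation on the skeletal mesh and posts the Wwise movement sound.
; Tick smooths actor rotation through interpolation and, when flagged, starts a timeline updating the hit bone's physics blend weight.
; Functions set that bone to full physics blend and launch the Medusa for knockback.
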(event `self.ReceiveBeginPlay`
  ;[1 1 1] Begin Play
  ;[1 1 1] Startin Physics Animation settings
  (`self.Startin Physics Animation settings`)
  (`AkGameplayStatics.PostEvent` "/Game/Audio/Enemy/Meduse/Medusa_Movement.Medusa_Movement" self))

(event `Startin Physics Animation settings`
  (bind _physicalanimation (`self.PhysicalAnimation`))
  (bind _bonename (`self.BoneName`))
  (bind _mesh (`self.Mesh`))
  ;[1 1 1] Startin Physics Animation settings
  (`PhysicalAnimationComponent.SetSkeletalMeshComponent` _physicalanimation (`self.Mesh`))
  (`PhysicalAnimationComponent.ApplyPhysicalAnimationSettingsBelow` _physicalanimation _bonename (make `PhysicalAnimationData` true 10.0 10.0 10.0 10.0 10.0) false)
  (`SkeletalMeshComponent.SetAllBodiesBelowSimulatePhysics` _mesh _bonename false true)
  (`SkeletalMeshComponent.SetAllBodiesBelowPhysicsBlendWeight` _mesh _bonename 0.0 false false))

(event `Deactivate Physics Anim`
  ;[1 1 1] Deactivate Physics Anim
  (if (`self.Physics Anim`)
    (`Timeline|Timeline_0` :!via `PlayFromStart`
      (:`Update`
        (`SkeletalMeshComponent.SetAllBodiesBelowPhysicsBlendWeight` (`self.Mesh`) (`self.Bone Hit`) 0.0 false true)
        (set `self.Physics Anim` false)))))

(event `self.ReceiveTick`
  (params (DeltaSeconds :type "Float (single-precision)"))
  ;[1 1 1] Event Tick
  ;[1 1 1] Interp Rotation
  (`self.InterpRotation`)
  ;[1 1 1] Deactivate Physics Anim
  (`self.Deactivate Physics Anim`))

(event `InterpRotation`
  (bind _returnvalue (`KismetMathLibrary.RInterpTo` (`self.PreActorRotation`) (`self.K2_GetActorRotation`) (`GameplayStatics.GetWorldDeltaSeconds`) 20.0))
  ;[1 1 1] SmoothRotation
  (`self.K2_SetActorRotation` _returnvalue)
  (set `self.PreActorRotation` _returnvalue))

(event `self.DamageCollider.OnComponentBeginOverlap`
  (params (OverlappedComponent :type "PrimitiveComponent Object Reference") (OtherActor :type "Actor Object Reference") (OtherComp :type "PrimitiveComponent Object Reference") (OtherBodyIndex :type Integer) (bFromSweep :type Boolean) (SweepResult :type "HitResult Structure (by ref)"))
  ;[1 1 1] Damage Main Character and apply KnockBack
  (bind _asmain_character_bp (cast `/Game/Blueprint/MainCharacter/MainCharacter_BP` OtherActor))
  (bind _output_get (set `self.RefToMainCharacter` _asmain_character_bp))
  (`GameplayStatics.ApplyDamage` _output_get 10.0 null null "/Script/Engine.DamageType")
  (`/Game/Blueprint/MainCharacter/MainCharacter_BP.KnockBack` (`self.RefToMainCharacter`)))

(fn `Activate Physics Anim`
  (`SkeletalMeshComponent.SetAllBodiesBelowPhysicsBlendWeight` (`self.Mesh`) (`self.Bone Hit`) 1.0 false true))

(fn `Knock Back`
  (params (KnockBackDirection :type "Vector Structure"))
  (`self.LaunchCharacter` KnockBackDirection true true))

(fn `UserConstructionScript`)