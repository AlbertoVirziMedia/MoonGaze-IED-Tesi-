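; Behavior tree service that finds a target for the Esploratori melee enemy on each tick.
; A sphere trace around the controlled pawn gathers nearby pawns, and those within range are written to the blackboard as target and location.
; Farther hits need a clear visibility line trace from a raised origin, otherwise the target key is cleared.
; Each hit overwrites the previous result, and an empty trace leaves the blackboard untouched.
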(event `self.ReceiveTick`
  (params (OwnerActor :type "Actor Object Reference") (DeltaSeconds :type "Float (single-precision)"))
  ;[1 1 1] Check for players in rang
  (bind _asesploratori_melee_aicontroller_bp (cast `/Game/Blueprint/Enemy/Esploratori/Melee/EsploratoriMeleeAIController_BP` OwnerActor))
  (bind _output_get (set `self.EMAIController` _asesploratori_melee_aicontroller_bp))
  (bind _returnvalue (`Actor.K2_GetActorLocation` (`Controller.K2_GetPawn` _output_get)))
  (bind _output_get_2 (set `self.SelfLocation` _returnvalue))
  (bind (_outhits _returnvalue_2) (`KismetSystemLibrary.SphereTraceMultiForObjects` _output_get_2 (+ _returnvalue (0.0 0.0 0.0)) 2000.0 (`|MakeArray` "ObjectTypeQuery3" :!type "EObjectTypeQuery Enum") false (`|MakeArray` (`Controller.K2_GetPawn` (`self.EMAIController`)) :!type "Actor Object Reference")))
  (if _returnvalue_2
    (for _array_element _outhits
      (bind _asesploratori_melee_character_bp (cast `/Game/Blueprint/Enemy/Esploratori/Melee/EsploratoriMeleeCharacter_BP` (`Controller.K2_GetPawn` (`self.EMAIController`))))
      (bind (_bblockinghit _binitialoverlap _time _distance _location _impactpoint _normal _impactnormal _physmat _hitactor) (`GameplayStatics.BreakHitResult` _array_element))
      (bind _distancetoenemy (`/Game/Blueprint/Enemy/Esploratori/Melee/EsploratoriMeleeCharacter_BP.GetDistanceToEnemy` _asesploratori_melee_character_bp _hitactor))
      (if (< _distancetoenemy 2000.0)
        (`BTFunctionLibrary.SetBlackboardValueAsObject` (`self.TargetKey`) _hitactor)
        (bind _returnvalue_3 (`Actor.K2_GetActorLocation` _hitactor))
        (`BTFunctionLibrary.SetBlackboardValueAsVector` (`self.TargetLocation`) _returnvalue_3)
        (`|MultiGate` false true)
        (else
          (bind _outhit (`KismetSystemLibrary.LineTraceSingle` (+ (`self.SelfLocation`) (0.0 0.0 96.0)) _returnvalue_3 "TraceTypeQuery1" false (`|MakeArray` (`Controller.K2_GetPawn` (`self.EMAIController`)) :!type "Actor Object Reference")))
          (bind (_bblockinghit_2 _binitialoverlap_2 _time_2 _distance_2 _location_2 _impactpoint_2 _normal_2 _impactnormal_2 _physmat_2 _hitactor_2) (`GameplayStatics.BreakHitResult` _outhit))
          (if (== _hitactor_2 _hitactor)
            (`BTFunctionLibrary.SetBlackboardValueAsObject` (`self.TargetKey`) _hitactor_2)
            (`BTFunctionLibrary.SetBlackboardValueAsVector` (`self.TargetLocation`) (`Actor.K2_GetActorLocation` _hitactor_2))
            (else
              (`BTFunctionLibrary.SetBlackboardValueAsObject` (`self.TargetKey`)))))))))