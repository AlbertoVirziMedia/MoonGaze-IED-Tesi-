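; Behavior tree task that picks a random patrol destination for the Esploratori melee enemy.
; On execute, it applies the patrol walk speed to the character, then looks for a random reachable point within the patrol radius around its location.
; It writes that point to the PatrolLocation blackboard key, falling back to the pawn's current location if none is found.
; The task fails only when the controlled pawn is not an Esploratori melee character.
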(event `self.ReceiveExecuteAI`
  (params (OwnerController :type "AIController Object Reference") (ControlledPawn :type "Pawn Object Reference"))
  (bind _returnvalue (`Actor.K2_GetActorLocation` ControlledPawn))
  (bind (_randomlocation _returnvalue_2) (`NavigationSystemV1.K2_GetRandomReachablePointInRadius` _returnvalue (`self.PatrolRadius`) null null))
  ;[1 1 1] Find Random position around the character
  (bind _asesploratori_melee_character_bp (cast `/Game/Blueprint/Enemy/Esploratori/Melee/EsploratoriMeleeCharacter_BP` ControlledPawn)
    (:`then`
      (`/Game/Blueprint/Enemy/Esploratori/Melee/EsploratoriMeleeCharacter_BP.UpdateWalkSpeed` _asesploratori_melee_character_bp (`self.PatrolSpeed`))
      (if _returnvalue_2
        (bind _returnvalue_3 (`AIBlueprintHelperLibrary.GetBlackboard` _asesploratori_melee_character_bp))
        (`BlackboardComponent.SetValueAsVector` _returnvalue_3 (`self.PatrolLocation`) _randomlocation)
        (`self.FinishExecute` true)
        (else
          (`BlackboardComponent.SetValueAsVector` _returnvalue_3 (`self.PatrolLocation`) _returnvalue)
          (`self.FinishExecute` true))))
    (:`CastFailed`
      (`self.FinishExecute` false))))