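; AI controller for the melee Esploratori enemy that sets up its blackboard and records the controlled pawn's starting location on BeginPlay.
; Construction initializes HasLineOfSight to false, and StartEnemyTimer resets that flag and clears TargetKey.
; The perception update event is empty: the logic that targets the sensed player or starts a delayed line-of-sight loss timer is disconnected and never runs.
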(event `self.AIPerceptionComp.OnTargetPerceptionUpdated`
  (params (Actor :type "Actor Object Reference") (Stimulus :type "AIStimulus Structure")))

(event `StartEnemyTimer`
  ;[1 1 1] if Not, Start the Timer for he have lost line of sight
  (`BlackboardComponent.SetValueAsBool` (`self.EMBlackboardComp`) (`self.HasLineOfSight`) false)
  (`BlackboardComponent.SetValueAsObject` (`self.EMBlackboardComp`) (`self.TargetKey`) null))

(event `self.ReceiveBeginPlay`
  ;[1 1 1] Get Initial location
  (`self.UseBlackboard` null)
  (`BlackboardComponent.SetValueAsVector` (`self.EMBlackboardComp`) (`self.SelfLocation`) (`self.K2_GetActorLocation` (`self.K2_GetPawn`))))

(fn `UserConstructionScript`
  (`BlackboardComponent.SetValueAsBool` (`self.EMBlackboardComp`) (`self.HasLineOfSight`) false))