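; Melee Esploratori enemy character, with functions for attacking, walk speed, distance checks, knockback and blood hit particles.
; Physical animation simulates bones at BeginPlay; PhysicsHit raises the hit bone's blend weight, and the PhysicsAnim flag triggers a timeline driving it.
; Tick also smooths actor rotation.
; Attack enables DamageCollider during the combat montage and damages the last actor that overlapped it.
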(event `self.ReceiveBeginPlay`
  ;[1 1 1] Begin Play
  ;[1 1 1] Physics Animation Stating Value
  (`self.Physics Animation starting value`))

(event `Physics Animation starting value`
  (bind _bonename (`self.BoneName`))
  (bind _physicalanimation (`self.PhysicalAnimation`))
  (bind _mesh (`self.Mesh`))
  ;[1 1 1] Physics Animation Stating Value
  (`PhysicalAnimationComponent.SetSkeletalMeshComponent` _physicalanimation (`self.Mesh`))
  (`PhysicalAnimationComponent.ApplyPhysicalAnimationSettingsBelow` _physicalanimation _bonename (make `PhysicalAnimationData` false 10.0 10.0 10.0 10.0 10.0) false)
  (`SkeletalMeshComponent.SetAllBodiesBelowSimulatePhysics` _mesh _bonename true false)
  (`SkeletalMeshComponent.SetAllBodiesBelowPhysicsBlendWeight` _mesh _bonename 0.0 false true))

(event `self.ReceiveTick`
  (params (DeltaSeconds :type "Float (single-precision)"))
  ;[1 1 1] Event Tick
  ;[1 1 1] Smooth Rotation
  (`self.InterpRotationToMain`)
  ;[1 1 1] Deactivate Physics Anim
  (`self.Deactivate Physics Anim`))

(event `InterpRotationToMain`
  (bind _returnvalue (`KismetMathLibrary.RInterpTo` (`self.PreActorRotation`) (`self.K2_GetActorRotation`) (`GameplayStatics.GetWorldDeltaSeconds`) 20.0))
  ;[1 1 1] Smooth Rotation
  (`self.K2_SetActorRotation` _returnvalue)
  (set `self.PreActorRotation` _returnvalue))

(event `Deactivate Physics Anim`
  ;[1 1 1] Deactivate Physics Anim
  (if (`self.PhysicsAnim`)
    (bind (_direction _newtrack_0) (`Timeline|Timeline_1` :!via `PlayFromStart`)
      (:`Update`
        (`SkeletalMeshComponent.SetAllBodiesBelowPhysicsBlendWeight` (`self.Mesh`) (`self.BoneHit`) _newtrack_0 false true)
        (set `self.PhysicsAnim` false)))))

(event `self.DamageCollider.OnComponentBeginOverlap`
  (params (OverlappedComponent :type "PrimitiveComponent Object Reference") (OtherActor :type "Actor Object Reference") (OtherComp :type "PrimitiveComponent Object Reference") (OtherBodyIndex :type Integer) (bFromSweep :type Boolean) (SweepResult :type "HitResult Structure (by ref)"))
  (set `self.MainCharacterActor` OtherActor))

(event `self.DamageCollider.OnComponentEndOverlap`
  (params (OverlappedComponent :type "PrimitiveComponent Object Reference") (OtherActor :type "Actor Object Reference") (OtherComp :type "PrimitiveComponent Object Reference") (OtherBodyIndex :type Integer)))

(fn `Attack`
  (if (`AnimInstance.Montage_IsPlaying` (`SkeletalMeshComponent.GetAnimInstance` (`self.Mesh`)) "/Game/ENemy/Animation/EnemyCombatMontage.EnemyCombatMontage")
    (`PrimitiveComponent.SetCollisionEnabled` (`self.DamageCollider`) "QueryOnly")
    (`GameplayStatics.ApplyDamage` (`self.MainCharacterActor`) 50.0 null null "/Script/Engine.DamageType")
    (else
      (`PrimitiveComponent.SetCollisionEnabled` (`self.DamageCollider`) "NoCollision"))))

(fn `GetDistanceToEnemy`
  (params (OtherActor :type "Actor Object Reference"))
  (returns (DistanceToEnemy :type "Float (double-precision)"))
  (if (!= OtherActor null)
    (return (`self.GetDistanceTo` OtherActor self))))

(fn `KnockBack`
  (params (KnockBackDirection :type "Vector Structure"))
  (`self.LaunchCharacter` KnockBackDirection true true))

(fn `Physics Hit`
  (`SkeletalMeshComponent.SetAllBodiesBelowPhysicsBlendWeight` (`self.Mesh`) (`self.BoneHit`) 1.0 false true))

(fn `SpawnHitParticle`
  (params (HitPosition :type "Vector Structure"))
  (`GameplayStatics.SpawnEmitterAtLocation` "/Game/VFX/DrippingBlood/P_SpriteBlood.P_SpriteBlood" HitPosition))

(fn `UpdateWalkSpeed`
  (params (NewWalkSpeed :type "Float (double-precision)"))
  (set `CharacterMovementComponent.MaxWalkSpeed` NewWalkSpeed (`self.CharacterMovement`)))

(fn `UserConstructionScript`)