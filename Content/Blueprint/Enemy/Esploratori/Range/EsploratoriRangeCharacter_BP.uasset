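; Character Blueprint for the ranged Esploratori enemy, handling its physical animation, staff melee hits, knockback and death.
; BeginPlay sets up partial-body physical animation and caches the player; Tick smooths rotation and runs a timeline on hit-bone physics blending.
; Staff overlaps knock the player back, dealing damage only when unblocked, once per overlap.
; Helpers cover speed, distance and blood particles, while Destroy animates a disintegration material before removing the actor.
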(event `self.ReceiveBeginPlay`
  ;[1 1 1] BeginPlay
  ;[1 1 1] PhysicsAnimationStartingValue
  (`self.PhysicsAnimationStartingValue`)
  ;[1 1 1] SetRefToMainCharacter
  (`self.SetRefToMainCharacter`)
  (`PrimitiveComponent.SetCollisionEnabled` (`self.DamageColliderBastone`) "NoCollision"))

(event `PhysicsAnimationStartingValue`
  (bind _physicalanimation (`self.PhysicalAnimation`))
  (bind _bonename (`self.BoneName`))
  (bind _mesh (`self.Mesh`))
  ;[1 1 1] PhysicsAnimationStartingValue
  (`PhysicalAnimationComponent.SetSkeletalMeshComponent` _physicalanimation (`self.Mesh`))
  (`PhysicalAnimationComponent.ApplyPhysicalAnimationSettingsBelow` _physicalanimation _bonename (make `PhysicalAnimationData` false 10.0 10.0 10.0 10.0 10.0) false)
  (`SkeletalMeshComponent.SetAllBodiesBelowSimulatePhysics` _mesh _bonename true false)
  (`SkeletalMeshComponent.SetAllBodiesBelowPhysicsBlendWeight` _mesh _bonename 0.0 false true))

(event `SetRefToMainCharacter`
  ;[1 1 1] SetRefToMainCharacter
  (set `self.RefToMainCharacter` (`GameplayStatics.GetPlayerPawn` 0)))

(event `self.ReceiveTick`
  (params (DeltaSeconds :type "Float (single-precision)"))
  ;[1 1 1] Event Tick
  ;[1 1 1] SmoothRotation
  (`self.SmoothRotation`)
  ;[1 1 1] DeactivatePhysicsAnim
  (`self.DeactivatePhysicsAnim`))

(event `SmoothRotation`
  (bind _returnvalue (`KismetMathLibrary.RInterpTo` (`self.PreActorRotation`) (`self.K2_GetActorRotation`) (`GameplayStatics.GetWorldDeltaSeconds`) 20.0))
  ;[1 1 1] SmoothRotation
  (`self.K2_SetActorRotation` _returnvalue)
  (set `self.PreActorRotation` _returnvalue))

(event `DeactivatePhysicsAnim`
  ;[1 1 1] DeactivatePhysicsAnim
  (if (`self.PhysicsAnim`)
    (`Timeline|Timeline_0` :!via `PlayFromStart`
      (:`Update`
        (`SkeletalMeshComponent.SetAllBodiesBelowPhysicsBlendWeight` (`self.Mesh`) (`self.BoneHit`) 0.0 false true)
        (set `self.PhysicsAnim` false)))))

(event `self.DamageColliderBastone.OnComponentBeginOverlap`
  (params (OverlappedComponent :type "PrimitiveComponent Object Reference") (OtherActor :type "Actor Object Reference") (OtherComp :type "PrimitiveComponent Object Reference") (OtherBodyIndex :type Integer) (bFromSweep :type Boolean) (SweepResult :type "HitResult Structure (by ref)"))
  ;[1 1 1] MeleeDamageCollider
  (bind _asmain_character_bp (cast `/Game/Blueprint/MainCharacter/MainCharacter_BP` OtherActor))
  (bind _output_get (set `self.RefToMainCharacterActor` _asmain_character_bp))
  (if (not (`MainCharacter.bIsBlocking` _output_get))
    (`/Engine/EditorBlueprintResources/StandardMacros.DoOnce` false :!label _label
      (:`Completed`
        (`GameplayStatics.ApplyDamage` _output_get 10.0 null null "/Script/Engine.DamageType"))))
  ;[1 1 1] Knockback
  (`/Game/Blueprint/MainCharacter/MainCharacter_BP.KnockBack` _output_get (`SceneComponent.GetForwardVector` (`self.Mesh`)))
  (set `/Game/Blueprint/MainCharacter/MainCharacter_BP.Kria_Enemies_Hits` self _output_get))

(event `self.DamageColliderBastone.OnComponentEndOverlap`
  (params (OverlappedComponent :type "PrimitiveComponent Object Reference") (OtherActor :type "Actor Object Reference") (OtherComp :type "PrimitiveComponent Object Reference") (OtherBodyIndex :type Integer))
  ;[1 1 1] MeleeDamageCollider
  (goto _label :!via `Reset`))

(event `Destroy`
  (bind _mesh (`self.Mesh`))
  ;[1 1 1] Disintegration
  (bind _returnvalue (`PrimitiveComponent.CreateDynamicMaterialInstance` _mesh 0 "/Game/VFX/DissolvingEffect/MI_disintegration_Inst.MI_disintegration_Inst" "None"))
  (bind _counter (`/Engine/EditorBlueprintResources/StandardMacros.Do N` (`PrimitiveComponent.GetNumMaterials` _mesh))
    (:`Exit`
      (`PrimitiveComponent.SetMaterial` _mesh _counter _returnvalue)
      (`MaterialInstanceDynamic.SetVectorParameterValue` _returnvalue "Location" (`KismetMathLibrary.Conv_VectorToLinearColor` (`self.K2_GetActorLocation` (`self.RefToMainCharacter`))))
      (bind (_direction _newtrack_0) (`Timeline|Disintegration` :!via `PlayFromStart`)
        (:`Update`
          (`MaterialInstanceDynamic.SetScalarParameterValue` _returnvalue "Amount" _newtrack_0))
        (:`Finished`
          (`self.K2_DestroyActor`))))))

(fn `GetDistanceToEnemy`
  (params (OtherActor :type "Actor Object Reference"))
  (returns (DistanceToEnemy :type "Float (double-precision)"))
  (if (!= OtherActor null)
    (return (`self.GetDistanceTo` OtherActor self))))

(fn `KnockBack`
  (params (KnockBackDirection :type "Vector Structure"))
  (`self.LaunchCharacter` KnockBackDirection true true))

(fn `SpawnHitParticle`
  (`GameplayStatics.SpawnEmitterAtLocation` (`|GetArrayItem` (`|MakeArray` (`self.SangueFront1`) (`self.SangueFront3`) (`self.SangueFront4`)) (`KismetMathLibrary.RandomInteger` 4)) (`SceneComponent.GetSocketLocation` (`self.Mesh`) "VFXSocket")))

(fn `UpdateWalkSpeed`
  (params (NewWalkSpeed :type "Float (double-precision)"))
  (set `CharacterMovementComponent.MaxWalkSpeed` NewWalkSpeed (`self.CharacterMovement`)))

(fn `UserConstructionScript`)