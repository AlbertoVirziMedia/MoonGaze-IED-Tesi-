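; ERBullet_BP is the spinning projectile of the ranged Esploratori enemy, damaging the player on overlap.
; A blocking player takes horizontal knockback against their mesh's forward vector; otherwise damage applies only once per bullet.
; Any other overlap plays a Wwise ground-impact sound at the sweep location.
; When projectile movement stops, rotation halts, the cube simulates physics and damage collision switches off.
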(event `self.ReceiveTick`
  (params (DeltaSeconds :type "Float (single-precision)")))

(event `self.ReceiveBeginPlay`
  ;[1 1 1] Starting Collision
  (`PrimitiveComponent.SetCollisionEnabled` (`self.DamageCollider`) "QueryOnly"))

(event `self.ProjectileMovement.OnProjectileStop`
  (params (ImpactResult :type "HitResult Structure (by ref)"))
  ;[1 1 1] After Collision Stop rotation
  (set `RotatingMovementComponent.RotationRate` (struct) (`self.RotatingMovement`))
  (`PrimitiveComponent.SetSimulatePhysics` (`self.Cube`) true)
  (`PrimitiveComponent.SetCollisionEnabled` (`self.DamageCollider`) "NoCollision"))

(event `self.DamageCollider.OnComponentBeginOverlap`
  (params (OverlappedComponent :type "PrimitiveComponent Object Reference") (OtherActor :type "Actor Object Reference") (OtherComp :type "PrimitiveComponent Object Reference") (OtherBodyIndex :type Integer) (bFromSweep :type Boolean) (SweepResult :type "HitResult Structure (by ref)"))
  ;[1 1 1] Collision
  (bind _asmain_character_bp (cast `/Game/Blueprint/MainCharacter/MainCharacter_BP` OtherActor)
    (:`then`
      (if (`MainCharacter.bIsBlocking` _asmain_character_bp)
        (`/Game/Blueprint/MainCharacter/MainCharacter_BP.KnockBack` _asmain_character_bp (* (`SceneComponent.GetForwardVector` (`Character.Mesh` _asmain_character_bp)) (-1.0 -1.0 0.0)))
        (else
          (`/Engine/EditorBlueprintResources/StandardMacros.DoOnce` false
            (:`Completed`
              (`GameplayStatics.ApplyDamage` _asmain_character_bp 10.0 null null "/Script/Engine.DamageType"))))))
    (:`CastFailed`
      (bind _returnvalue (`AkGameplayStatics.SpawnAkComponentAtLocation` "/Game/Audio/Enemy/Esploratori/Range/Esploratori_Fionda_Impact_Ground.Esploratori_Fionda_Impact_Ground" (`.Location` (`GameplayStatics.BreakHitResult` SweepResult))))
      (`AkGameObject.PostAssociatedAkEvent` :`self` _returnvalue))))

(fn `UserConstructionScript`)