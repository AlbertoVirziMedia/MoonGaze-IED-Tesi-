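; Character Blueprint for the Liocarpio crab enemy, handling melee hits on the player, hit reactions and disintegration.
; Two damage colliders, disabled at start, knock the player back, dealing damage only when unblocked, gated once per overlap.
; Tick smooths actor rotation and fades bone physics blend through a timeline for physical-animation hit reactions.
; Timelines drive a dissolve material located at the player, forward or reversed; Attack only checks montage state, without acting.
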(event `self.ReceiveBeginPlay`
  ;[1 1 1] Begin Play
  ;[1 1 1] SetInitialPhysicalAnimData
  (`self.SetInitialPhysicalAnimData`)
  ;[1 1 1] SetRefToMainCharacter
  (`self.SetRefToMainCharacter`)
  ;[1 1 1] DeactivateDamageCollider
  (`self.DeactivateDamageCollider`))

(event `DeactivateDamageCollider`
  ;[1 1 1] DeactivateDamageCollider
  (`PrimitiveComponent.SetCollisionEnabled` (`self.DamageCollider`) "NoCollision")
  (`PrimitiveComponent.SetCollisionEnabled` (`self.DamageColliderDx`) "NoCollision"))

(event `SetRefToMainCharacter`
  ;[1 1 1] SetRefToMainCharacter
  (set `self.RefToManCharacterPawn` (`GameplayStatics.GetPlayerPawn` 0)))

(event `SetInitialPhysicalAnimData`
  (bind _physicalanimation (`self.PhysicalAnimation`))
  (bind _mesh (`self.Mesh`))
  (bind _bonename (`self.BoneName`))
  ;[1 1 1] SetInitialPhysicalAnimData
  (`PhysicalAnimationComponent.SetSkeletalMeshComponent` _physicalanimation (`self.Mesh`))
  (`PhysicalAnimationComponent.ApplyPhysicalAnimationSettingsBelow` _physicalanimation _bonename (make `PhysicalAnimationData` false 10.0 10.0 10.0 10.0 10.0) false)
  (`SkeletalMeshComponent.SetAllBodiesBelowSimulatePhysics` _mesh _bonename true false)
  (`SkeletalMeshComponent.SetAllBodiesBelowPhysicsBlendWeight` _mesh _bonename 0.0 false true))

(event `self.ReceiveTick`
  (params (DeltaSeconds :type "Float (single-precision)"))
  ;[1 1 1] Event Tick
  ;[1 1 1] InterCustomRotation
  (`self.InterCustomRotation`)
  ;[1 1 1] Deactivate Physics Anim
  (`self.DeactivatePhysicsAnim`))

(event `InterCustomRotation`
  (bind _returnvalue (`KismetMathLibrary.RInterpTo` (`self.PreActorRotation`) (`self.K2_GetActorRotation`) (`GameplayStatics.GetWorldDeltaSeconds`) 15.0))
  ;[1 1 1] InterCustomRotation
  (`self.K2_SetActorRotation` _returnvalue)
  (set `self.PreActorRotation` _returnvalue))

(event `DeactivatePhysicsAnim`
  ;[1 1 1] Deactivate Physics Anim
  (if (`self.PhysicsAnim`)
    (bind (_direction _newtrack_0) (`Timeline|Timeline_0` :!via `PlayFromStart`)
      (:`Update`
        (`SkeletalMeshComponent.SetAllBodiesBelowPhysicsBlendWeight` (`self.Mesh`) (`self.BoneHit`) _newtrack_0 false true)
        (set `self.PhysicsAnim` false)))))

(event `self.DamageCollider.OnComponentBeginOverlap`
  (params (OverlappedComponent :type "PrimitiveComponent Object Reference") (OtherActor :type "Actor Object Reference") (OtherComp :type "PrimitiveComponent Object Reference") (OtherBodyIndex :type Integer) (bFromSweep :type Boolean) (SweepResult :type "HitResult Structure (by ref)"))
  (bind _reftomaincharacter (`self.RefToMainCharacter`))
  ;[1 1 1] Sx and Dx Damage Collider
  (bind _asmain_character_bp (cast `/Game/Blueprint/MainCharacter/MainCharacter_BP` OtherActor))
  (bind _output_get (set `self.RefToMainCharacter` _asmain_character_bp))
  (if (`MainCharacter.bIsBlocking` _output_get)
    (`/Game/Blueprint/MainCharacter/MainCharacter_BP.BlockSound` _output_get)
    (else
      (`/Engine/EditorBlueprintResources/StandardMacros.DoOnce` false :!label _label
        (:`Completed`
          (`GameplayStatics.ApplyDamage` _output_get 10.0 null null "/Script/Engine.DamageType")
          (`/Game/Blueprint/MainCharacter/MainCharacter_BP.SpawnHitParticle` _output_get "None")))))
  (`/Game/Blueprint/MainCharacter/MainCharacter_BP.KnockBack` _reftomaincharacter (* (`SceneComponent.GetForwardVector` (`Character.Mesh` (`self.RefToMainCharacter`))) (-1.0 -1.0 0.0)))
  (set `/Game/Blueprint/MainCharacter/MainCharacter_BP.Kria_Enemies_Hits` self _reftomaincharacter))

(event `self.DamageColliderDx.OnComponentBeginOverlap`
  (params (OverlappedComponent :type "PrimitiveComponent Object Reference") (OtherActor :type "Actor Object Reference") (OtherComp :type "PrimitiveComponent Object Reference") (OtherBodyIndex :type Integer) (bFromSweep :type Boolean) (SweepResult :type "HitResult Structure (by ref)"))
  (bind _reftomaincharacter (`self.RefToMainCharacter`))
  ;[1 1 1] Sx and Dx Damage Collider
  (bind _asmain_character_bp (cast `/Game/Blueprint/MainCharacter/MainCharacter_BP` OtherActor))
  (bind _output_get (set `self.RefToMainCharacter` _asmain_character_bp))
  (if (`MainCharacter.bIsBlocking` _output_get)
    (`/Game/Blueprint/MainCharacter/MainCharacter_BP.BlockSound` _output_get)
    (else
      (`/Engine/EditorBlueprintResources/StandardMacros.DoOnce` false :!label _label_2
        (:`Completed`
          (`GameplayStatics.ApplyDamage` _output_get 10.0 null null "/Script/Engine.DamageType")
          (`/Game/Blueprint/MainCharacter/MainCharacter_BP.SpawnHitParticle` _output_get "None")))))
  (`/Game/Blueprint/MainCharacter/MainCharacter_BP.KnockBack` _reftomaincharacter (* (`SceneComponent.GetForwardVector` (`Character.Mesh` (`self.RefToMainCharacter`))) (-1.0 -1.0 0.0)))
  (set `/Game/Blueprint/MainCharacter/MainCharacter_BP.Kria_Enemies_Hits` self _reftomaincharacter))

(event `self.DamageCollider.OnComponentEndOverlap`
  (params (OverlappedComponent :type "PrimitiveComponent Object Reference") (OtherActor :type "Actor Object Reference") (OtherComp :type "PrimitiveComponent Object Reference") (OtherBodyIndex :type Integer))
  ;[1 1 1] Sx and Dx Damage Collider
  (goto _label :!via `Reset`))

(event `self.DamageColliderDx.OnComponentEndOverlap`
  (params (OverlappedComponent :type "PrimitiveComponent Object Reference") (OtherActor :type "Actor Object Reference") (OtherComp :type "PrimitiveComponent Object Reference") (OtherBodyIndex :type Integer))
  ;[1 1 1] Sx and Dx Damage Collider
  (goto _label_2 :!via `Reset`))

(event `Destroy`
  (bind _mesh (`self.Mesh`))
  ;[1 1 1] Disintegration
  (bind _returnvalue (`PrimitiveComponent.CreateDynamicMaterialInstance` _mesh 0 "/Game/VFX/DissolvingEffect/MI_disintegration_Inst.MI_disintegration_Inst" "None"))
  (bind _counter (`/Engine/EditorBlueprintResources/StandardMacros.Do N` (`PrimitiveComponent.GetNumMaterials` _mesh))
    (:`Exit`
      (`PrimitiveComponent.SetMaterial` _mesh _counter _returnvalue)
      (`MaterialInstanceDynamic.SetVectorParameterValue` _returnvalue "Location" (`KismetMathLibrary.Conv_VectorToLinearColor` (`self.K2_GetActorLocation` (`self.RefToManCharacterPawn`))))
      (bind (_direction _newtrack_0) (`Timeline|Disintegration` :!via `PlayFromStart`)
        (:`Update`
          (`MaterialInstanceDynamic.SetScalarParameterValue` _returnvalue "Amount" _newtrack_0))))))

(event `ReverseDisintegration`
  (bind _mesh (`self.Mesh`))
  (bind _returnvalue (`PrimitiveComponent.CreateDynamicMaterialInstance` _mesh 0 "/Game/VFX/DissolvingEffect/MI_disintegration_Inst.MI_disintegration_Inst" "None"))
  (bind _counter (`/Engine/EditorBlueprintResources/StandardMacros.Do N` (`PrimitiveComponent.GetNumMaterials` _mesh))
    (:`Exit`
      (`PrimitiveComponent.SetMaterial` _mesh _counter _returnvalue)
      (`MaterialInstanceDynamic.SetVectorParameterValue` _returnvalue "Location" (`KismetMathLibrary.Conv_VectorToLinearColor` (`self.K2_GetActorLocation` (`self.RefToManCharacterPawn`))))
      (bind (_direction _newtrack_0) (`Timeline|Reverse` :!via `PlayFromStart`)
        (:`Update`
          (`MaterialInstanceDynamic.SetScalarParameterValue` _returnvalue "Amount" _newtrack_0))
        (:`Finished`
          (`PrimitiveComponent.SetMaterial` (`self.Mesh`) 0 "/Game/Materials/Enemies/Granchio_Liocarpio/M_Granchio_Main.M_Granchio_Main"))))))

(fn `Attack`
  (bind _returnvalue (`SkeletalMeshComponent.GetAnimInstance` (`self.Mesh`)))
  (if (`AnimInstance.Montage_IsPlaying` _returnvalue "/Game/ENemy/Liocarpio/Animazioni/LiocarpioCombatMontage.LiocarpioCombatMontage")
    (if (== (`AnimInstance.Montage_GetCurrentSection` _returnvalue "/Game/ENemy/Liocarpio/Animazioni/LiocarpioCombatMontage.LiocarpioCombatMontage") "FastAttack")
      _)))

(fn `GetDistanceToEnemy`
  (params (OtherActor :type "Actor Object Reference"))
  (returns (DistanceToEnemy :type "Float (double-precision)"))
  (if (!= OtherActor null)
    (return (`self.GetDistanceTo` self OtherActor))))

(fn `KnockBack`
  (params (KnockBackDirection :type "Vector Structure"))
  (`self.LaunchCharacter` (* KnockBackDirection (10.0 10.0 10.0)) true true))

(fn `Physics Hit`
  (`SkeletalMeshComponent.SetAllBodiesBelowPhysicsBlendWeight` (`self.Mesh`) (`self.BoneHit`) 1.0 false true))

(fn `SpawnHitParticle`
  (`GameplayStatics.SpawnEmitterAtLocation` (`|GetArrayItem` (`|MakeArray` (`self.SangueFront6`) (`self.SangueFront7`) (`self.SangueFront8`) (`self.SangueFront9`)) (`KismetMathLibrary.RandomInteger` 4)) (`SceneComponent.GetSocketLocation` (`self.Mesh`) "VFXSocket")))

(fn `UpdateWalkSpeed`
  (params (NewWalkSpeed :type "Float (double-precision)"))
  (set `CharacterMovementComponent.MaxWalkSpeed` NewWalkSpeed (`self.CharacterMovement`)))

(fn `UserConstructionScript`)