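; Custom camera actor that rides along the spline of a referenced track actor once activated.
; Tick watches ActiveCamera and fires the move once, playing a timeline at a rate of one over Duration.
; The timeline alpha maps to spline distance, setting world location and rotation with a fixed 90-degree offset.
; CartStartOffset sets the timeline time, but the following PlayFromStart restarts it from zero.
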(event `self.ReceiveTick`
  (params (DeltaSeconds :type "Float (single-precision)"))
  (if (`self.ActiveCamera`)
    (`/Engine/EditorBlueprintResources/StandardMacros.DoOnce` false
      (:`Completed`
        (`self.MOveAlongTheTrack`)))))

(event `MOveAlongTheTrack`
  (bind _cameratimeline (`self.CameraTimeline`))
  (bind _returnvalue (`KismetMathLibrary.Lerp` 0.0 (`SplineComponent.GetSplineLength` (`/Game/Blueprint/Component/CameraTrack.Track` (`self.TrackRef`))) (`self.Alpha`)))
  (`TimelineComponent.SetPlayRate` _cameratimeline (/ 1.0 (`self.Duration`)))
  (`TimelineComponent.SetNewTime` _cameratimeline (`self.CartStartOffset`))
  (bind (_direction _alpha) (`Timeline|CameraTimeline` :!via `PlayFromStart`)
    (:`Update`
      (set `self.Alpha` _alpha)
      (`self.K2_SetActorLocationAndRotation` (`SplineComponent.GetLocationAtDistanceAlongSpline` (`/Game/Blueprint/Component/CameraTrack.Track` (`self.TrackRef`)) _returnvalue "World") (`KismetMathLibrary.ComposeRotators` (`SplineComponent.GetRotationAtDistanceAlongSpline` (`/Game/Blueprint/Component/CameraTrack.Track` (`self.TrackRef`)) _returnvalue "World") (struct :`Yaw` 90.0))))))

(fn `UserConstructionScript`)