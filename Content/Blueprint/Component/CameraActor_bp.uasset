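; CameraActor_bp is an actor that plays a camera sequence through an array of camera actors, then returns the view to the player character.
; On BeginPlay it resets the index after a short delay and caches the MainCharacter_BP pawn.
; MoveCamera disables character movement, blends to each camera with aspect-ratio constraint off, and calls itself after a configurable delay.
; After the last camera, it blends back more slowly and calls RestartMovement on the character.
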(event `RefToMainCharacter`
  ;[1 1 1] RefToMainCharacter
  (bind _asmain_character_bp (cast `/Game/Blueprint/MainCharacter/MainCharacter_BP` (`GameplayStatics.GetPlayerPawn` 0)))
  (set `self.RefToMainChar` _asmain_character_bp))

(event `self.ReceiveBeginPlay`
  ;[1 1 1] Set Initial Index
  (`KismetSystemLibrary.Delay` 0.2)
  (set `self.index` 0)
  ;[1 1 1] RefToMainCharacter
  (`self.RefToMainCharacter`))

(event `MoveCamera`
  (bind _output (`|GetArrayItem` (`self.CameraActor`) (`self.index`)))
  (if (< (`self.index`) (`KismetArrayLibrary.Array_Length` (`self.CameraActor`)))
    ;[1 1 1] Disable Character Ref
    (`CharacterMovementComponent.DisableMovement` (`Character.CharacterMovement` (`self.RefToMainChar`)))
    ;[1 1 1] Bland Camera Position
    (`CameraComponent.SetConstraintAspectRatio` (`CameraActor.CameraComponent` _output) false)
    (`PlayerController.SetViewTargetWithBlend` (`GameplayStatics.GetPlayerController` 0) _output 2.0 "VTBlend_EaseInOut" 2.0 true)
    (`KismetSystemLibrary.Delay` (`self.delay`))
    (set `self.index` (+ (`self.index`) 1))
    (`self.MoveCamera`)
    (else
      ;[1 1 1] ReturnToMainCamera
      (`PlayerController.SetViewTargetWithBlend` (`GameplayStatics.GetPlayerController` 0) (`GameplayStatics.GetPlayerCharacter` 0) 6.0 "VTBlend_EaseInOut" 2.0 true)
      (`/Game/Blueprint/MainCharacter/MainCharacter_BP.RestartMovement` (`self.RefToMainChar`)))))

(fn `UserConstructionScript`)