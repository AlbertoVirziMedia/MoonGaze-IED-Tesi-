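; ArenaSpawnEmitter is a component that turns its owning StaticMeshActor into a toggleable magic-wall arena barrier.
; On BeginPlay it caches the owner and disables the mesh's collision.
; The activate function spawns the P_MagicWallArena particle effect at the owner's location and enables query and physics collision.
; The deactivate function only disables collision; despite its name, it does not stop the spawned emitter.
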(event `self.ReceiveBeginPlay`
  ;[1 1 1] Set Ref to Owner
  (bind _asstatic_mesh_actor (cast `StaticMeshActor` (`self.GetOwner`)))
  (bind _output_get (set `self.RefToOwner` _asstatic_mesh_actor))
  ;[1 1 1] Deactivate Collision O Begin Play
  (`PrimitiveComponent.SetCollisionEnabled` (`StaticMeshActor.StaticMeshComponent` _output_get) "NoCollision"))

(fn `SpawnEmitterandActivateCollider`
  (bind _reftoowner (`self.RefToOwner`))
  (`GameplayStatics.SpawnEmitterAtLocation` "/Game/VFX/MagicWall/P_MagicWallArena.P_MagicWallArena" (`Actor.K2_GetActorLocation` _reftoowner))
  (`PrimitiveComponent.SetCollisionEnabled` (`StaticMeshActor.StaticMeshComponent` _reftoowner) "QueryAndPhysics"))

(fn `StopEmitterandDeactivateCollider`
  (`PrimitiveComponent.SetCollisionEnabled` (`StaticMeshActor.StaticMeshComponent` (`self.RefToOwner`)) "NoCollision"))