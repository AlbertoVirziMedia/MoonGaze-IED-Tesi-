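; Hover component that keeps its owning actor floating above surfaces using physics forces.
; On BeginPlay it enables physics simulation on the owner's first primitive component.
; Each tick it traces straight down in world space and, on a hit, pushes along the surface normal with force fading linearly to zero at full trace length.
; A hit also applies linear and angular damping, which is never reset when the trace misses.
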(event `self.ReceiveBeginPlay`
  (bind _output_get (set `self.PrimitiveComponent` (`|GetArrayItem` (`Actor.K2_GetComponentsByClass` (`self.GetOwner`) "/Script/Engine.PrimitiveComponent"))))
  (`PrimitiveComponent.SetSimulatePhysics` _output_get true))

(event `self.ReceiveTick`
  (params (DeltaSeconds :type "Float (single-precision)"))
  (bind _returnvalue (`self.K2_GetComponentLocation`))
  (bind _primitivecomponent (`self.PrimitiveComponent`))
  (bind (_outhit _returnvalue_2) (`KismetSystemLibrary.LineTraceSingle` :`Start` _returnvalue :`End` (- _returnvalue (`KismetMathLibrary.MakeVector` 0.0 0.0 (`self.TraceLenght`))) :`TraceChannel` "TraceTypeQuery2" :`DrawDebugType` "ForDuration"))
  (if _returnvalue_2
    (bind (_bblockinghit _binitialoverlap _time _distance _location _impactpoint _normal _impactnormal) (`GameplayStatics.BreakHitResult` _outhit))
    (`PrimitiveComponent.AddForce` _primitivecomponent (* _impactnormal (`KismetMathLibrary.Lerp` (`self.HoverForce`) 0.0 (/ (`KismetMathLibrary.VSize` (- _location (`self.K2_GetComponentLocation`))) (`self.TraceLenght`)))) "None" false)
    (`PrimitiveComponent.SetLinearDamping` _primitivecomponent (`self.LinearDamping`))
    (`PrimitiveComponent.SetAngularDamping` _primitivecomponent (`self.AngularDamping`))))