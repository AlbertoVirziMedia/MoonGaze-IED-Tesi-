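; Player character Blueprint that wires input to dash, sword attack and target-system calls, and drives the character's Wwise audio.
; Attacking toggles sword collision and damages the last enemy cached by sword overlap, on press rather than on overlap.
; BeginPlay starts health and level music events; Tick moves the listener to AkListener with camera rotation and feeds Health to an RTPC.
; R self-damages; jump, movement and blocking calls are unconnected.
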(event `InputAction|Dash`
  (params (Key :type "Key Structure"))
  ;[1 1 1] Dash
  (:`Pressed`
    (`self.Dash`)
    ;[1 1 1] WWIse Audio Dash Implementation
    (bind _returnvalue (`AkGameplayStatics.SpawnAkComponentAtLocation` "/Game/Audio/MainCharacter/Kria_Dash.Kria_Dash" (`SceneComponent.K2_GetComponentLocation` (`self.Mesh`))))
    (`AkGameObject.PostAssociatedAkEvent` :`self` _returnvalue))
  (:`Released`
    (`self.StopDashing`)))

(event `InputAction|Attack`
  (params (Key :type "Key Structure"))
  ;[1 1 1] Attack Function
  (:`Pressed`
    (`self.Attack`)
    (set `self.bIsAttacking` true)
    ;[1 1 1] Attack
    (if (`self.bIsAttacking`) :!label _label
      (`PrimitiveComponent.SetCollisionEnabled` (`self.SwordAttack`) "QueryOnly")
      (`GameplayStatics.ApplyDamage` (stale `self.SwordAttack.OnComponentBeginOverlap` _asenemy_character_bp) 10.0 null null "/Script/Engine.DamageType")
      (else
        (`PrimitiveComponent.SetCollisionEnabled` (`self.SwordAttack`) "NoCollision"))))
  (:`Released`
    (`self.AttackEnd`)
    (set `self.bIsAttacking` false)
    (goto _label)))

(event `self.SwordAttack.OnComponentBeginOverlap`
  (params (OverlappedComponent :type "PrimitiveComponent Object Reference") (OtherActor :type "Actor Object Reference") (OtherComp :type "PrimitiveComponent Object Reference") (OtherBodyIndex :type Integer) (bFromSweep :type Boolean) (SweepResult :type "HitResult Structure (by ref)"))
  ;[1 1 1] Attack
  (if (`self.bIsAttacking`)
    (bind _asenemy_character_bp (cast `/Game/Blueprint/Enemy/EnemyCharacter_BP` OtherActor))))

(event `Key|Gamepad_RightTrigger`
  (params (Key :type "Key Structure"))
  ;[1 1 1] Target System
  (:`Pressed`
    (`MainTargetSystemComponent.TargetActor` (`self.MainTargetSystem`) :!label _label_2)))

(event `Key|C`
  (params (Key :type "Key Structure"))
  ;[1 1 1] Target System
  (:`Pressed`
    (goto _label_2)))

(event `self.ReceiveTick`
  (params (DeltaSeconds :type "Float (single-precision)"))
  ;[1 1 1] Third Person Listener (WWise)
  (`PlayerController.SetAudioListenerOverride` (`GameplayStatics.GetPlayerController` 0) null (`SceneComponent.K2_GetComponentLocation` (`self.AkListener`)) (`PlayerCameraManager.GetCameraRotation` (`GameplayStatics.GetPlayerCameraManager` 0)))
  ;[1 1 1] Set RTPC Kria_Health
  (`AkGameplayStatics.SetRTPCValue` "Kria_Health" (`self.Health`) 20)
  ;[1 1 1] Get the Distance From ENemy
  (bind _asenemy_character_bp (cast `/Game/Blueprint/Enemy/EnemyCharacter_BP` (`self.EnemyTargetRefToDistance`))))

(event `self.ReceiveBeginPlay`
  ;[1 1 1] Start Ak Event Kria_Health
  (`AkGameplayStatics.PostEvent` "/Game/Audio/MainCharacter/Kria_Health.Kria_Health" self)
  ;[1 1 1] Start Ak Event Music (Implement Switch State)
  (`AkGameplayStatics.SetState` "Figthing_Variable" "No_Fight")
  (`AkGameplayStatics.PostEvent` "/Game/Audio/Music/Start_Level.Start_Level" self))

(event `Key|R`
  (params (Key :type "Key Structure"))
  (:`Pressed`
    (`GameplayStatics.ApplyDamage` self 10.0 null null "/Script/Engine.DamageType")))

(fn `UserConstructionScript`)