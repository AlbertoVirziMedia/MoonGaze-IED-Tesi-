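; Main game mode Blueprint that starts all ambient sounds on play and reloads BlockOut_Level when the player is killed.
; Every tick it inserts the alive flags of FirstArena-tagged Liocarpio enemies into an array, never clearing it.
; It only prints whether all flags are false, as arena-clear debug output.
; Disconnected nodes hold unused logic for removing the MagicWall barrier and respawning the player.
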(event `self.ReceiveBeginPlay`
  ;[1 1 1] Start all Ambient Sound
  (`AkGameplayStatics.StartAllAmbientSounds`))

(event `self.ReceiveTick`
  (params (DeltaSeconds :type "Float (single-precision)"))
  (`self.CheckIfTheEnemysAreAlive`)
  (set `self.AllTrue` true)
  (for _array_element (`self.EnemyAlive`)
    (if _array_element
      (set `self.AllTrue` false)
      (break)))
  (if (`self.AllTrue`)
    (`KismetSystemLibrary.PrintString` "alltrue")
    (else
      (`KismetSystemLibrary.PrintString` "allfalse"))))

(event `CheckIfTheEnemysAreAlive`
  (bind _outactors (`GameplayStatics.GetAllActorsOfClassWithTag` "/Game/Blueprint/Enemy/Liocarpio/LiocarpioCharacter_BP.LiocarpioCharacter_BP_C" "FirstArena"))
  (for (_array_element _array_index) _outactors
    (bind _asliocarpio_character_bp (cast `/Game/Blueprint/Enemy/Liocarpio/LiocarpioCharacter_BP` _array_element))
    (`KismetArrayLibrary.Array_Insert` (`self.EnemyAlive`) (`GenericEnemyCharacter.bEnemyIsAlive` _asliocarpio_character_bp) _array_index)))

(fn `OnPlayerKilled`
  (params (MainCharacter :type "/Game/Blueprint/MainCharacter/MainCharacter_BP Object Reference"))
  ;[1 1 1] Restart Function
  (`GameplayStatics.OpenLevel` "BlockOut_Level"))

(fn `UserConstructionScript`)