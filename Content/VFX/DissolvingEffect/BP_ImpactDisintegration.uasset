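; Actor whose cube disintegrates and is then destroyed when the MainCharacter hits it.
; BeginPlay creates a dynamic instance of the disintegration material on the cube.
; The first hit passes a DoOnce before the character cast, sets the material's Location to the character's position, and starts a timeline driving Amount.
; A delay off the timeline update disables collision after two seconds, and timeline completion destroys the actor.
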(event `self.ReceiveBeginPlay`
  (bind _returnvalue (`PrimitiveComponent.CreateDynamicMaterialInstance` (`self.Cube`) 0 "/Game/VFX/DissolvingEffect/MI_disintegration_Inst.MI_disintegration_Inst" "None"))
  (set `self.Dyn_Mat` _returnvalue))

(event `self.Cube.OnComponentHit`
  (params (HitComponent :type "PrimitiveComponent Object Reference") (OtherActor :type "Actor Object Reference") (OtherComp :type "PrimitiveComponent Object Reference") (NormalImpulse :type "Vector Structure") (Hit :type "HitResult Structure (by ref)"))
  (bind _dyn_mat (`self.Dyn_Mat`))
  (`/Engine/EditorBlueprintResources/StandardMacros.DoOnce` false
    (:`Completed`
      (cast `MainCharacter` OtherActor)
      (`MaterialInstanceDynamic.SetVectorParameterValue` _dyn_mat "Location" (`KismetMathLibrary.Conv_VectorToLinearColor` (`self.K2_GetActorLocation` OtherActor)))
      (bind (_direction _newtrack_0) (`Timeline|Timeline_0` :!via `PlayFromStart`)
        (:`Update`
          (`MaterialInstanceDynamic.SetScalarParameterValue` _dyn_mat "Amount" _newtrack_0)
          (`KismetSystemLibrary.Delay` 2.0)
          (`PrimitiveComponent.SetCollisionEnabled` (`self.Cube`) "NoCollision"))
        (:`Finished`
          (`self.K2_DestroyActor`))))))

(fn `UserConstructionScript`)