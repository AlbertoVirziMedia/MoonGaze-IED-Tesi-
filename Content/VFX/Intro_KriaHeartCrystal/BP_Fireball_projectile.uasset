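; Fireball projectile for the KriaHeartCrystal intro VFX that homes on the first BP_Projectile_Target found at BeginPlay.
; A timeline scales a random per-spawn offset to bend the path.
; Tick interpolates toward just above the target and rotates using its velocity, with a loop-back that ramps speed to its cap within one frame.
; On arrival it deactivates the Fireball effect and destroys itself after a delay.
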(event `self.ReceiveBeginPlay`
  (bind _outactors (`GameplayStatics.GetAllActorsOfClass` "/Game/VFX/Intro_KriaHeartCrystal/BP_Projectile_Target.BP_Projectile_Target_C"))
  (set `self.Z` (`KismetMathLibrary.RandomFloatInRange` -2.0 2.0))
  (set `self.Y` (`KismetMathLibrary.RandomFloatInRange` -2.0 2.0))
  (set `self.X` (`KismetMathLibrary.RandomFloatInRange` -3.0 3.0))
  (bind (_direction _newtrack_0) (`Timeline|Timeline_0`)
    (:`Update`
      (`SceneComponent.K2_AddWorldOffset` (`self.DefaultSceneRoot`) (* _newtrack_0 (`KismetMathLibrary.MakeVector` (`self.X`) (`self.Y`) (`self.Z`))) false false))))

(event `self.ReceiveTick`
  (params (DeltaSeconds :type "Float (single-precision)"))
  (bind _returnvalue (`KismetMathLibrary.Fraction` DeltaSeconds))
  (bind _returnvalue_2 (`SceneComponent.K2_GetComponentLocation` (`self.DefaultSceneRoot`)))
  (bind _output_get (set `self.Time` (+ (`self.Time`) 10.0) :!label _label))
  (bind _staticmeshcomponent (`StaticMeshActor.StaticMeshComponent` (`|GetArrayItem` (stale `self.ReceiveBeginPlay` _outactors))))
  (bind _returnvalue_3 (+ (`SceneComponent.K2_GetComponentLocation` _staticmeshcomponent) (0.0 0.0 25.0)))
  (`SceneComponent.K2_SetWorldLocation` (`self.DefaultSceneRoot`) (`KismetMathLibrary.VInterpTo_Constant` _returnvalue_2 _returnvalue_3 _returnvalue _output_get) false false)
  (`SceneComponent.K2_SetWorldRotation` (`self.DefaultSceneRoot`) (`KismetMathLibrary.RInterpTo_Constant` (`SceneComponent.K2_GetComponentRotation` (`self.DefaultSceneRoot`)) (`KismetMathLibrary.MakeRotator` (.x (`SceneComponent.GetComponentVelocity` _staticmeshcomponent)) (.y (`SceneComponent.GetComponentVelocity` _staticmeshcomponent)) (.z (`SceneComponent.GetComponentVelocity` _staticmeshcomponent))) _returnvalue 1000.0) false false)
  (while (<= _output_get 1000.0)
    (goto _label))
  (if (== _returnvalue_2 _returnvalue_3)
    (`ActorComponent.Deactivate` (`self.Fireball`))
    (`KismetSystemLibrary.Delay` 1.5)
    (`self.K2_DestroyActor`)))

(fn `UserConstructionScript`)