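; BP_Vomit is a short-lived acid vomit hazard that damages the player on contact, likely part of a boss's acid ball attack.
; On BeginPlay it spawns a randomly sized vomit decal from a dynamic material instance at the mesh location, then destroys itself after a fixed delay.
; Mesh overlap applies one-off damage to MainCharacter_BP and calls PlayerInAcid, with PlayerNotInAcid called when overlap ends.
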(event `self.ReceiveBeginPlay`
  (bind _returnvalue (`KismetMaterialLibrary.CreateDynamicMaterialInstance` "/Game/VFX/Blood_Decal/M_Blood_Decal_Inst_VOMITO.M_Blood_Decal_Inst_VOMITO"))
  (`GameplayStatics.SpawnDecalAtLocation` _returnvalue (`KismetMathLibrary.Conv_DoubleToVector` (`KismetMathLibrary.RandomFloatInRange` 1.0 5.0)) (`SceneComponent.K2_GetComponentLocation` (`self.vomit_mesh`)))
  (`KismetSystemLibrary.Delay` 5.0)
  (`self.K2_DestroyActor`))

(event `self.vomit_mesh.OnComponentBeginOverlap`
  (params (OverlappedComponent :type "PrimitiveComponent Object Reference") (OtherActor :type "Actor Object Reference") (OtherComp :type "PrimitiveComponent Object Reference") (OtherBodyIndex :type Integer) (bFromSweep :type Boolean) (SweepResult :type "HitResult Structure (by ref)"))
  ;[1 1 1] Damage Character
  (bind _asmain_character_bp (cast `/Game/Blueprint/MainCharacter/MainCharacter_BP` OtherActor))
  (`GameplayStatics.ApplyDamage` _asmain_character_bp 20.0 null null "/Script/Engine.DamageType")
  (`/Game/Blueprint/MainCharacter/MainCharacter_BP.PlayerInAcid` _asmain_character_bp))

(event `self.vomit_mesh.OnComponentEndOverlap`
  (params (OverlappedComponent :type "PrimitiveComponent Object Reference") (OtherActor :type "Actor Object Reference") (OtherComp :type "PrimitiveComponent Object Reference") (OtherBodyIndex :type Integer))
  ;[1 1 1] Damage Character
  (bind _asmain_character_bp (cast `/Game/Blueprint/MainCharacter/MainCharacter_BP` OtherActor))
  (`/Game/Blueprint/MainCharacter/MainCharacter_BP.PlayerNotInAcid` _asmain_character_bp))

(fn `UserConstructionScript`)