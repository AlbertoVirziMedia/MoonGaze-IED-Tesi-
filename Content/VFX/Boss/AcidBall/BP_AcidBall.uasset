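; Boss acid ball projectile that arcs toward the player's position and leaves a BP_Vomit pool.
; On BeginPlay, if active, it builds a three-point spline with a raised midpoint, aimed below the player's position at launch.
; Timelines move and deform the sphere along it while downward traces find the ground.
; On finish it spawns a randomly scaled pool at the spline-end hit, or under the player as fallback, then destroys itself.
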(event `self.ReceiveBeginPlay`
  (bind _acidball_trajectory (`self.AcidBall_Trajectory`))
  (bind _parabola_time (`self.Parabola Time`))
  (bind _trace_vomit_location (`self.Trace Vomit Location`))
  (bind _returnvalue (`SplineComponent.GetLocationAtSplinePoint` (`self.AcidBall_Trajectory`) 3 "World"))
  (bind _returnvalue_2 (`KismetMathLibrary.MakeVector` (`KismetMathLibrary.RandomFloatInRange` 1.0 2.0) (`KismetMathLibrary.RandomFloatInRange` 1.0 2.0) 1.0))
  (bind _returnvalue_3 (`SceneComponent.K2_GetComponentLocation` (`self.DefaultSceneRoot`)))
  (bind _returnvalue_4 (`SceneComponent.K2_GetComponentLocation` (`Character.CapsuleComponent` (`GameplayStatics.GetPlayerCharacter` 0))))
  (bind _returnvalue_5 (`SceneComponent.K2_GetComponentLocation` (`Character.CapsuleComponent` (`GameplayStatics.GetPlayerCharacter` 0))))
  ;[1 1 1] Condition
  (if (`self.AcidBall Active`)
    ;[1 1 1] Set Spline Points in World Space (0 Actor Loc, 1 Middle, 2 Player Loc)
    (`SplineComponent.SetSplinePoints` (`self.AcidBall_Trajectory`) (`|MakeArray` _returnvalue_3 (`KismetMathLibrary.MakeVector` (`KismetMathLibrary.SafeDivide` (+ (.x _returnvalue_3) (.x _returnvalue_4)) 2.0) (`KismetMathLibrary.SafeDivide` (+ (.y _returnvalue_3) (.y _returnvalue_4)) 2.0) (* (+ (.z _returnvalue_3) (.z _returnvalue_4)) (`self.Arc Z Mult`))) (+ _returnvalue_4 (0.0 0.0 -200.0))) "World" true)
    ;[1 1 1] Movement Along Spline
    (bind (_direction _alpha) (`Timeline|Timeline_1` :`NewTime` _parabola_time)
      (:`Update`
        ;;[0.3173 0.205 1] Scale Along Spline
        (bind (_direction_2 _scale_x _scale_y _scale_z) (`Timeline|Scale deformation` :`NewTime` _parabola_time)
          (:`Update`
            (bind _returnvalue_6 (* (`SplineComponent.GetSplineLength` _acidball_trajectory) _alpha))
            (`SceneComponent.K2_SetWorldTransform` (`self.SphereBone`) (`KismetMathLibrary.MakeTransform` (`SplineComponent.GetLocationAtDistanceAlongSpline` _acidball_trajectory _returnvalue_6 "World") (`SplineComponent.GetRotationAtDistanceAlongSpline` _acidball_trajectory _returnvalue_6 "World") (3.0 3.0 3.0)) true false)
            (`SceneComponent.SetWorldScale3D` (`self.SphereBone`) (* (`KismetMathLibrary.MakeVector` _scale_z _scale_x _scale_y) 5.0))
            ;[1 1 1] Im LineTracing both the Last Spline Point and the Player Location
            (bind _outhit (`KismetSystemLibrary.LineTraceSingle` :`Start` _returnvalue :`End` (`KismetMathLibrary.MakeVector` (.x _returnvalue) (.y _returnvalue) (- (.z _returnvalue) 100000.0)) :`TraceChannel` "TraceTypeQuery1" :`bTraceComplex` true :`DrawDebugType` "Persistent"))
            (`KismetSystemLibrary.PrintString` (`KismetStringLibrary.Conv_VectorToString` (`.ImpactPoint` (`GameplayStatics.BreakHitResult` _outhit))) false true (struct :`G` 1.0 :`B` 0.080142 :`A` 1.0))
            (set `self.Trace Vomit Location` (`.ImpactPoint` (`GameplayStatics.BreakHitResult` _outhit)))
            (`/Engine/EditorBlueprintResources/StandardMacros.DoOnce` false
              (:`Completed`
                (bind _outhit_2 (`KismetSystemLibrary.LineTraceSingle` _returnvalue_5 (`KismetMathLibrary.MakeVector` (.x _returnvalue_5) (.y _returnvalue_5) (- (.z _returnvalue_5) 1000000.0)) "TraceTypeQuery1"))
                (bind _output_get (set `self.Player LineTraced Loc` (`.ImpactPoint` (`GameplayStatics.BreakHitResult` _outhit_2))))
                (`KismetSystemLibrary.PrintString` (`KismetStringLibrary.Conv_VectorToString` _output_get) false true (struct :`R` 1.0 :`G` 0.120615 :`A` 1.0)))))))
      (:`Finished`
        ;[1 1 1] Debug End Timeline
        (`KismetSystemLibrary.PrintString` "vomit and then destroy" false true (struct :`R` 1.0 :`G` 0.074582 :`A` 1.0))
        ;[1 1 1] Wether to spawn the Vomit pool at the character feet or at the linetraced down last spline point
        (if (<= (.z _trace_vomit_location) 1.0)
          (`|SpawnActorFromClass` "/Game/VFX/Boss/AcidBall/BP_Vomit.BP_Vomit_C" (`KismetMathLibrary.MakeTransform` (`self.Player LineTraced Loc`) (struct) _returnvalue_2) "AlwaysSpawn" "OverrideRootScale" null null)
          (else
            (`|SpawnActorFromClass` "/Game/VFX/Boss/AcidBall/BP_Vomit.BP_Vomit_C" (`KismetMathLibrary.MakeTransform` (- _trace_vomit_location (0.0 0.0 5.0)) (struct) _returnvalue_2) "AlwaysSpawn" "OverrideRootScale" null null)))
        (`self.K2_DestroyActor`)))))

(fn `UserConstructionScript`)